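; BP_Lumber is a woodmill building with state-dependent visuals and an animated saw.
; SetColorByState sets the Woodmill material: green or red by CanBePlaced while floating, the normal material when ready, with none assigned for processing or under construction.
; DoProcessing rotates the Saw by a fixed local increment on each call, independent of delta time.
; The event graph holds only disabled placeholder events.
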(fn `DoProcessing`
  (`SceneComponent.K2_AddLocalRotation` (`self.Saw`) (struct :`Pitch` 10.0) false false))

(fn `SetColorByState`
  (bind _result (`self.CanBePlaced`))
  (`PrimitiveComponent.SetMaterial` (`self.Woodmill`) 0 (select `/Game/Buildings/E_Building_State` (`self.State`) :`NewEnumerator0` (select `bool` _result :`false` "/Game/Materials/M_Woodmill_Red.M_Woodmill_Red" :`true` "/Game/Materials/M_Woodmill_Green.M_Woodmill_Green" :!type "MaterialInterface Object Reference") :`NewEnumerator1` "/Game/Materials/M_Woodmill.M_Woodmill")))

(fn `UserConstructionScript`
  (`parent.UserConstructionScript`))