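; Base Blueprint for resource buildings that have a worker and a processing cycle.
; On placement it runs the parent logic, then starts the loop on the BP_Worker held in its child actor component.
; StartProcessing and EndProcessing switch the state between PROCESSING and READY.
; While processing, Tick calls DoProcessing every frame, an empty hook that leaves the actual work to subclasses.
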(event `self.ReceiveTick`
  (params (DeltaSeconds :type "Float (single-precision)"))
  (`parent.ReceiveTick` DeltaSeconds)
  (switch `/Game/Buildings/E_Building_State` (`self.State`)
    (:`NewEnumerator2`
      (`self.DoProcessing`))))

(fn `DoProcessing`)

(fn `EndProcessing`
  (set `self.State` "NewEnumerator1"))

(fn `PlaceBuilding`
  (`parent.PlaceBuilding`)
  (bind _asbp_worker (cast `/Game/Characters/BP_Worker` (`ChildActorComponent.ChildActor` (`self.BP_Worker`))))
  (`/Game/Characters/BP_Worker.StartLoop` _asbp_worker))

(fn `StartProcessing`
  (set `self.State` "NewEnumerator2"))

(fn `UserConstructionScript`
  (`parent.UserConstructionScript`))