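; Game state Blueprint that holds the player's resource stockpile and handles building costs.
; On BeginPlay it creates the WBP_Top_Bar widget and seeds starting tree, rock and coin amounts.
; Amounts live in a map keyed by resource class, and SetResourceAmount updates both the map and the bar.
; AreCostsCovered checks a cost map against the stock, while PayForBuilding deducts it by adding negative amounts.
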(event `self.ReceiveBeginPlay`
  (bind _returnvalue (`|CreateWidget` "/Game/UI/WBP_Top_Bar.WBP_Top_Bar_C"))
  (`UserWidget.AddToViewport` _returnvalue 0)
  (set `self.ResourceBar` _returnvalue)
  (`self.SetResourceAmount` "/Game/Resources/BP_Tree.BP_Tree_C" 50)
  (`self.SetResourceAmount` "/Game/Resources/BP_Rock.BP_Rock_C" 30)
  (`self.SetResourceAmount` "/Game/Resources/BP_Coin.BP_Coin_C" 10))

(fn `AddResourceAmount`
  (params (resourceClass :type "/Game/Resources/BP_Resource Class Reference") (resourceAmount :type Integer))
  (bind (_value _returnvalue) (`BlueprintMapLibrary.Map_Find` (`self.ResourceMap`) resourceClass))
  (if _returnvalue
    (`self.SetResourceAmount` resourceClass (+ _value resourceAmount))
    (else
      (`self.SetResourceAmount` resourceClass resourceAmount))))

(fn `AreCostsCovered`
  (params (Costs :type "Map of /Game/Resources/BP_Resource Class Reference to Integer"))
  (returns (Result :type Boolean))
  (locals (TempResult :type Boolean :default true))
  (bind _keys (`BlueprintMapLibrary.Map_Keys` Costs))
  (for _array_element _keys
    ;[1 1 1] Check Every Resource
    (if (not (>= (`BlueprintMapLibrary.Map_Find` (`self.ResourceMap`) _array_element) (`BlueprintMapLibrary.Map_Find` Costs _array_element)))
      (set `local.TempResult` false)
      (break)))
  (return (`local.TempResult`)))

(fn `PayForBuilding`
  (params (Costs :type "Map of /Game/Resources/BP_Resource Class Reference to Integer"))
  (bind _keys (`BlueprintMapLibrary.Map_Keys` Costs))
  (for _array_element _keys
    (`self.AddResourceAmount` _array_element (* (`BlueprintMapLibrary.Map_Find` Costs _array_element) -1))))

(fn `SetResourceAmount`
  (params (resourceClass :type "/Game/Resources/BP_Resource Class Reference") (resourceAmount :type Integer))
  (`BlueprintMapLibrary.Map_Add` (`self.ResourceMap`) resourceClass resourceAmount)
  (`/Game/UI/WBP_Top_Bar.SetResourceAmount` (`self.ResourceBar`) resourceClass resourceAmount))

(fn `UserConstructionScript`)