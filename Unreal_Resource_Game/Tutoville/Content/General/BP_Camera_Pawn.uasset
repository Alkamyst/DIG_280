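; Camera pawn with a visible mouse cursor that pans, yaws and zooms through keyboard and mouse input.
; Each tick, Enhanced Input action values drive local-space movement and rotation scaled by delta time.
; Middle mouse drags pan and right mouse drags rotate, with middle taking priority.
; With neither button held, zoom changes the spring arm length, skipping any step outside its min/max range.
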(event `self.ReceiveBeginPlay`
  (set `PlayerController.bShowMouseCursor` true (`GameplayStatics.GetPlayerController` 0)))

(event `self.ReceiveTick`
  (params (DeltaSeconds :type "Float (single-precision)"))
  (bind (_returnvalue_x _returnvalue_y) (`KismetMathLibrary.BreakVector2D` (`|GetInputActionValue`)))
  (bind _maxcameraspeed (`self.MaxCameraSpeed`))
  (bind _springarm (`self.SpringArm`))
  (bind _returnvalue (+ (* (`|GetInputActionValue`) (`self.CameraZoomSpeed`) -1.0) (`SpringArmComponent.TargetArmLength` _springarm)))
  ;[1 1 1] Move By Keys
  (`self.K2_AddActorLocalOffset` (* (`KismetMathLibrary.GetForwardVector` (struct)) (`|GetInputActionValue`) (`self.MaxCameraSpeed`) DeltaSeconds))
  ;[1 1 1] Move By Keys
  (`self.K2_AddActorLocalOffset` (* (`self.MaxCameraSpeed`) (`KismetMathLibrary.GetRightVector` (struct)) (`|GetInputActionValue`) DeltaSeconds))
  ;[1 1 1] Rotate By Keys
  (`self.K2_AddActorLocalRotation` (`KismetMathLibrary.MakeRotator` 0.0 0.0 (* DeltaSeconds (`|GetInputActionValue`) (`self.CameraRotationSpeed`))))
  ;[1 1 1] Move By Mouse
  (if (`PlayerController.IsInputKeyDown` (`GameplayStatics.GetPlayerController` 0) "MiddleMouseButton")
    (`self.K2_AddActorLocalOffset` (+ (* (`KismetMathLibrary.GetForwardVector` (struct)) _maxcameraspeed _returnvalue_y DeltaSeconds) (* _returnvalue_x (`KismetMathLibrary.GetRightVector` (struct)) _maxcameraspeed DeltaSeconds)))
    (else
      ;[1 1 1] Rotate By Mouse
      (if (`PlayerController.IsInputKeyDown` (`GameplayStatics.GetPlayerController` 0) "RightMouseButton")
        (`self.K2_AddActorWorldRotation` (`KismetMathLibrary.MakeRotator` 0.0 0.0 (* _returnvalue_x (`self.CameraRotationSpeed`) DeltaSeconds)))
        (else
          ;[1 1 1] Zoom
          (if (and (<= _returnvalue (`self.MaxArmLength`)) (>= _returnvalue (`self.MinArmLength`)))
            (set `SpringArmComponent.TargetArmLength` _returnvalue _springarm)))))))

(fn `UserConstructionScript`)