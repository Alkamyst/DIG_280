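; BP_SphereHandler tracks how many Sphere_Blueprint actors have been destroyed and opens the level's Door_Blueprint once all are gone.
; At BeginPlay it counts the spheres and creates the WBP_Counter HUD widget with that total.
; HandleSphereDestroyed increments the kill count, restarts a "happy" timer and plays the widget's jump animation.
; Tick counts the timer down per frame, pushes both values to the widget and calls OpenDoor every frame once the goal is met.
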(event `self.ReceiveBeginPlay`
  (bind _outactors (`GameplayStatics.GetAllActorsOfClass` "/Game/Sphere_Blueprint.Sphere_Blueprint_C"))
  (bind _output_get (set `self.TotalSpheres` (`KismetArrayLibrary.Array_Length` _outactors)))
  (bind _returnvalue (`|CreateWidget` "/Game/Hud/WBP_Counter.WBP_Counter_C"))
  (bind _output_get_2 (set `self.BPCounter` _returnvalue))
  (`UserWidget.AddToViewport` _output_get_2 0)
  (set `/Game/Hud/WBP_Counter.MariosTotal` _output_get _output_get_2))

(event `self.ReceiveTick`
  (params (DeltaSeconds :type "Float (single-precision)"))
  (bind _happytimer (`self.HappyTimer`))
  (if (> _happytimer 0)
    (set `self.HappyTimer` (- _happytimer 1)))
  (set `/Game/Hud/WBP_Counter.HappyTimer` _happytimer (`self.BPCounter`))
  (set `/Game/Hud/WBP_Counter.MariosKilled` (`self.SpheresKilled`) (`self.BPCounter`))
  (if (>= (`self.SpheresKilled`) (`self.TotalSpheres`))
    (bind _returnvalue (`GameplayStatics.GetActorOfClass` "/Game/Models/Door/Door_Blueprint.Door_Blueprint_C"))
    (`/Game/Models/Door/Door_Blueprint.OpenDoor` _returnvalue)))

(fn `HandleSphereDestroyed`
  (set `self.HappyTimer` (`self.HappyTimerValue`))
  (set `self.SpheresKilled` (+ (`self.SpheresKilled`) 1))
  (`/Game/Hud/WBP_Counter.PlayJumpAnimation` (`self.BPCounter`)))

(fn `UserConstructionScript`)