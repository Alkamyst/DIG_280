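; BP_Dragon is a damageable dragon enemy that reacts to hits from BP_FirstPersonProjectile.
; Each hit subtracts health and plays a hurt or death sound, with a hit montage only while not flying.
; Exact health values drive the FlyingAnimStart and Die flags, starting flight after early damage.
; At zero health it spawns a BP_Star set to load FinalMap, then destroys itself.
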(event `self.ReceiveHit`
  (params (MyComp :type "PrimitiveComponent Object Reference") (Other :type "Actor Object Reference") (OtherComp :type "PrimitiveComponent Object Reference") (bSelfMoved :type Boolean) (HitLocation :type "Vector Structure") (HitNormal :type "Vector Structure") (NormalImpulse :type "Vector Structure") (Hit :type "HitResult Structure (by ref)"))
  (bind _returnvalue (`self.GetTransform`))
  (cast `/Game/FirstPerson/Blueprints/BP_FirstPersonProjectile` Other)
  (if (not (`self.FlyingAnimStart`))
    (`|PlayMontage` (`self.Mesh`) "/Game/FourEvilDragonsPBR/Animations/DragonTheSoulEater/GetHitAnim_Montage.GetHitAnim_Montage"
      (:`then`
        _)))
  (bind _output_get (set `self.Health` (- (`self.Health`) 10.0)))
  (if (> _output_get 0.0)
    (if (== (`KismetMathLibrary.RandomInteger` 2) 0)
      (`GameplayStatics.PlaySoundAtLocation` "/Game/Sounds/PacMan/Hurt2.Hurt2" (`self.K2_GetActorLocation`) (struct) 1.0 1.0 0.0 null null null null)
      (else
        (`GameplayStatics.PlaySoundAtLocation` "/Game/Sounds/PacMan/Hurt.Hurt" (`self.K2_GetActorLocation`) (struct) 1.0 1.0 0.0 null null null null)))
    (else
      (`GameplayStatics.PlaySoundAtLocation` "/Game/Sounds/PacMan/Die.Die" (`self.K2_GetActorLocation`) (struct) 1.0 1.0 0.0 null null null null)))
  (if (== _output_get 90.0)
    (set `self.FlyingAnimStart` true)
    (set `self.Die` false)
    (elif (== _output_get 0.0)
      (set `self.FlyingAnimStart` false)
      (set `self.Die` true)
      (bind _returnvalue_2 (`|SpawnActorFromClass` "/Game/Models/Star/BP_Star.BP_Star_C" (`KismetMathLibrary.MakeTransform` (`KismetMathLibrary.MakeVector` (.x (.location _returnvalue)) (.y (.location _returnvalue)) 100.0)) "Undefined" "MultiplyWithRoot" null null))
      (set `/Game/Models/Star/BP_Star.Level Name` "FinalMap" _returnvalue_2)
      (`self.K2_DestroyActor`)
      (elif (== _output_get -50.0)
        (set `self.Health` 0.0)
        (set `self.FlyingAnimStart` false)
        (set `self.Die` false)))))

(fn `UserConstructionScript`)