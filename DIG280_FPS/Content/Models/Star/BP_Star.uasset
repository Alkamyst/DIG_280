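; BP_Star is a spinning star actor that acts as a level goal, either advancing to another level or ending the game with a win.
; Tick adds a fixed yaw step every frame, so spin speed depends on frame rate.
; Any Hit destroys the star and clears all widgets, without checking what struck it.
; The FinalStar flag then selects the WBP_YouWin screen with a fanfare, otherwise it opens the level named in LevelName.
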(event `self.ReceiveTick`
  (params (DeltaSeconds :type "Float (single-precision)"))
  (bind (_returnvalue_roll _returnvalue_pitch _returnvalue_yaw) (`KismetMathLibrary.BreakRotator` (`self.K2_GetActorRotation`)))
  (`self.K2_SetActorRotation` (`KismetMathLibrary.MakeRotator` 0.0 0.0 (+ _returnvalue_yaw 5.0))))

(event `self.ReceiveHit`
  (params (MyComp :type "PrimitiveComponent Object Reference") (Other :type "Actor Object Reference") (OtherComp :type "PrimitiveComponent Object Reference") (bSelfMoved :type Boolean) (HitLocation :type "Vector Structure") (HitNormal :type "Vector Structure") (NormalImpulse :type "Vector Structure") (Hit :type "HitResult Structure (by ref)"))
  (`self.K2_DestroyActor`)
  (`WidgetLayoutLibrary.RemoveAllWidgets`)
  (if (`self.FinalStar`)
    (bind _returnvalue (`|CreateWidget` "/Game/Hud/WBP_YouWin.WBP_YouWin_C"))
    (`UserWidget.AddToViewport` _returnvalue 0)
    (`GameplayStatics.PlaySound2D` "/Game/Sounds/Star_Fanfare.Star_Fanfare" 1.0 1.0 0.0 null null)
    (else
      (`GameplayStatics.OpenLevel` (`self.Level Name`)))))

(fn `UserConstructionScript`)