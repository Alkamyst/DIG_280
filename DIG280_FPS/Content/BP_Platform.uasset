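; BP_Platform is a moving platform actor that travels between its placed location and that location plus MoveableOffset.
; BeginPlay caches both endpoints and sets the timeline play rate to the inverse of Timer.
; Tick calls Play on the timeline every frame, whose MovePlatform track drives a lerp between the endpoints without sweeping.
; The overlap event and construction script are empty.
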(event `self.ReceiveBeginPlay`
  (set `self.FirstPos` (`self.K2_GetActorLocation`))
  (set `self.LastPos` (+ (`self.FirstPos`) (`self.MoveableOffset`)))
  (`TimelineComponent.SetPlayRate` (`self.Timeline`) (/ 1.0 (`self.Timer`))))

(event `self.ReceiveTick`
  (params (DeltaSeconds :type "Float (single-precision)"))
  (bind (_direction _moveplatform) (`Timeline|Timeline`)
    (:`Update`
      (`self.K2_SetActorLocation` (`KismetMathLibrary.VLerp` (`self.FirstPos`) (`self.LastPos`) _moveplatform)))))

(fn `UserConstructionScript`)