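; Coin pickup actor that awards a coin to the player when Player_BP overlaps its sphere.
; It increments the player's coin count, or at 99 coins resets it to zero and grants an extra life.
; Each pickup copies the new values into the player's save object, writes it to a fixed slot, refreshes the HUD, plays a coin sound and destroys itself.
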(event `self.Sphere.OnComponentBeginOverlap`
  (params (OverlappedComponent :type "PrimitiveComponent Object Reference") (OtherActor :type "Actor Object Reference") (OtherComp :type "PrimitiveComponent Object Reference") (OtherBodyIndex :type Integer) (bFromSweep :type Boolean) (SweepResult :type "HitResult Structure (by ref)"))
  (bind _as_player_bp (`self.As Player BP`))
  (bind _as_player_bp_2 (`self.As Player BP`))
  (bind _as_player_save (`/Game/PlayerCharacter/Player_BP.As Player Save` (`self.As Player BP`)))
  (bind _as_player_save_2 (`/Game/PlayerCharacter/Player_BP.As Player Save` (`self.As Player BP`)))
  (bind _asplayer_bp (cast `/Game/PlayerCharacter/Player_BP` OtherActor))
  (bind _output_get (set `self.As Player BP` _asplayer_bp))
  (if (== (`/Game/PlayerCharacter/Player_BP.coins` _output_get) 99.0)
    (bind _output_get_2 (set `/Game/PlayerCharacter/Player_BP.lives` (+ (`/Game/PlayerCharacter/Player_BP.lives` _as_player_bp) 1.0) _as_player_bp))
    (`/Game/WidgetBlueprints/PlayerHud_WPB.Update Lives` (`/Game/PlayerCharacter/Player_BP.hudReference` (`self.As Player BP`)))
    (set `/Game/PlayerCharacter/PlayerSave.lives` _output_get_2 (`/Game/PlayerCharacter/Player_BP.As Player Save` (`self.As Player BP`)))
    (bind _output_get_3 (set `/Game/PlayerCharacter/Player_BP.coins` 0.0 _as_player_bp))
    (set `/Game/PlayerCharacter/PlayerSave.coins` _output_get_3 _as_player_save)
    (`GameplayStatics.SaveGameToSlot` _as_player_save "1")
    (else
      (bind _output_get_4 (set `/Game/PlayerCharacter/Player_BP.coins` (+ (`/Game/PlayerCharacter/Player_BP.coins` _as_player_bp_2) 1.0) _as_player_bp_2))
      (set `/Game/PlayerCharacter/PlayerSave.coins` _output_get_4 _as_player_save_2)
      (`GameplayStatics.SaveGameToSlot` _as_player_save_2 "1")))
  (`/Game/WidgetBlueprints/PlayerHud_WPB.Update Coins` (`/Game/PlayerCharacter/Player_BP.hudReference` (`self.As Player BP`)))
  (`GameplayStatics.PlaySoundAtLocation` "/Game/Sounds/RandomCoin_SC.RandomCoin_SC" (`self.K2_GetActorLocation`) (struct) 1.0 1.0 0.0 null null null null)
  (`self.K2_DestroyActor`))

(fn `UserConstructionScript`)