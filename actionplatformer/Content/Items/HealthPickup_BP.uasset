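; Health pickup actor that heals the player who touches it and is then consumed.
; An overlap on its sphere reacts only to Player_BP, and does nothing when that player's health equals its maximum.
; Otherwise it adds HealthToGive, clamped to max health, calls ShowHeart on the player's HUD reference with the truncated amount, plays a heal sound and destroys itself.
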(event `self.Sphere.OnComponentBeginOverlap`
  (params (OverlappedComponent :type "PrimitiveComponent Object Reference") (OtherActor :type "Actor Object Reference") (OtherComp :type "PrimitiveComponent Object Reference") (OtherBodyIndex :type Integer) (bFromSweep :type Boolean) (SweepResult :type "HitResult Structure (by ref)"))
  (bind _as_player_bp (`self.As Player BP`))
  (bind _as_player_bp_2 (`self.As Player BP`))
  (bind _asplayer_bp (cast `/Game/PlayerCharacter/Player_BP` OtherActor))
  (set `self.As Player BP` _asplayer_bp)
  (if (not (== (`/Game/PlayerCharacter/Player_BP.health` _as_player_bp_2) (`/Game/PlayerCharacter/Player_BP.maxHealth` _as_player_bp_2)))
    (set `/Game/PlayerCharacter/Player_BP.health` (`KismetMathLibrary.FClamp` (+ (`/Game/PlayerCharacter/Player_BP.health` _as_player_bp) (`self.HealthToGive`)) 1.0 (`/Game/PlayerCharacter/Player_BP.maxHealth` _as_player_bp)) _as_player_bp)
    (`/Game/WidgetBlueprints/PlayerHud_WPB.Show Heart` (`/Game/PlayerCharacter/Player_BP.hudReference` (`self.As Player BP`)) (`KismetMathLibrary.FTrunc` (`self.HealthToGive`)))
    (`GameplayStatics.PlaySoundAtLocation` "/Game/Sounds/heal.heal" (`self.K2_GetActorLocation`) (struct) 1.0 1.0 0.0 null null null null)
    (`self.K2_DestroyActor`)))

(fn `UserConstructionScript`)