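; ApplePickup_BP is a pickup that adds apples to the player's count when the player overlaps its sphere.
; If Player_BP is not already at max apples, it adds five, clamped to the maximum, and writes the count to the player's save object.
; It then saves to slot "1", refreshes the HUD, plays the Heal sound at its location and destroys itself.
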(event `self.Sphere.OnComponentBeginOverlap`
  (params (OverlappedComponent :type "PrimitiveComponent Object Reference") (OtherActor :type "Actor Object Reference") (OtherComp :type "PrimitiveComponent Object Reference") (OtherBodyIndex :type Integer) (bFromSweep :type Boolean) (SweepResult :type "HitResult Structure (by ref)"))
  (bind _as_player_bp (`self.As Player BP`))
  (bind _as_player_save (`/Game/PlayerCharacter/Player_BP.As Player Save` (`self.As Player BP`)))
  (bind _asplayer_bp (cast `/Game/PlayerCharacter/Player_BP` OtherActor))
  (bind _output_get (set `self.As Player BP` _asplayer_bp))
  (if (not (== (`/Game/PlayerCharacter/Player_BP.apples` _output_get) (`/Game/PlayerCharacter/Player_BP.maxApples` _output_get)))
    (bind _output_get_2 (set `/Game/PlayerCharacter/Player_BP.apples` (`KismetMathLibrary.Clamp` (+ (`/Game/PlayerCharacter/Player_BP.apples` _as_player_bp) 5) 1 (`/Game/PlayerCharacter/Player_BP.maxApples` _as_player_bp)) _as_player_bp))
    (set `/Game/PlayerCharacter/PlayerSave.apples` (`KismetMathLibrary.Conv_IntToDouble` _output_get_2) _as_player_save)
    (`GameplayStatics.SaveGameToSlot` _as_player_save "1")
    (`/Game/WidgetBlueprints/PlayerHud_WPB.UpdateApples` (`/Game/PlayerCharacter/Player_BP.hudReference` (`self.As Player BP`)))
    (`GameplayStatics.PlaySoundAtLocation` "/Game/Sounds/heal.heal" (`self.K2_GetActorLocation`) (struct) 1.0 1.0 0.0 null null null null)
    (`self.K2_DestroyActor`)))

(fn `UserConstructionScript`)