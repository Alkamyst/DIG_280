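; Mushroom ranged enemy that flips to face the player, fires projectiles and shows a health bar widget.
; Player overlap with its box starts a looping timer that plays the attack animation while alive and grounded; SpawnProjectile, not called here, spawns the shot.
; Damage updates the bar, then either pops it upward with a hit reaction or triggers death and delayed destruction.
; Animation states switch through JumpToNode calls on the AnimInstance.
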(event `self.ReceiveBeginPlay`
  (set `self.MaxHealth` (`self.Health`))
  (bind _asranged_enemy_health_bar_wbp (cast `/Game/WidgetBlueprints/RangedEnemyHealthBar_WBP` (`WidgetComponent.GetWidget` (`self.Widget`))))
  (bind _output_get (set `self.As Ranged Enemy Health Bar WBP` _asranged_enemy_health_bar_wbp))
  (set `/Game/WidgetBlueprints/RangedEnemyHealthBar_WBP.mushroomRef` self _output_get))

(event `self.ReceiveTick`
  (params (DeltaSeconds :type "Float (single-precision)"))
  (`self.HandleRotation`))

(event `HandleRotation`
  (bind _returnvalue_x (`KismetMathLibrary.BreakVector` (`KismetMathLibrary.GetDirectionUnitVector` (`self.K2_GetActorLocation` (`GameplayStatics.GetPlayerCharacter` 0)) (`self.K2_GetActorLocation`))))
  ;[1 1 1] Handle Rotation
  (if (`self.isDead`)
    _
    (elif (< _returnvalue_x 0.0)
      (`self.K2_SetActorRotation` (struct))
      (else
        (`self.K2_SetActorRotation` (struct :`Yaw` 180.0))))))

(event `self.ReceiveAnyDamage`
  (params (Damage :type "Float (single-precision)") (DamageType :type "DamageType Object Reference") (InstigatedBy :type "Controller Object Reference") (DamageCauser :type "Actor Object Reference"))
  ;[1 1 1] Handle Damage
  (bind _output_get (set `self.Health` (- (`self.Health`) Damage)))
  (set `self.enemyDamaged` true)
  (`/Game/WidgetBlueprints/RangedEnemyHealthBar_WBP.UpdateHealthBar` (`self.As Ranged Enemy Health Bar WBP`))
  (if (<= _output_get 0.0)
    (`PaperZDAnimInstance.JumpToNode` (`PaperZDAnimationComponent.AnimInstance` (`self.AnimationComponent`)) (`self.Death Jump Node`) "None")
    (set `self.isDead` true)
    (`PrimitiveComponent.SetCollisionProfileName` (`self.CapsuleComponent`) (`self.Damaged Jump Node`) true)
    (`SceneComponent.SetVisibility` (`self.Widget`) false false)
    (`KismetSystemLibrary.Delay` 3.0)
    (`self.K2_DestroyActor`)
    (else
      (`self.LaunchCharacter` (0.0 0.0 150.0) true true)
      (`PaperZDAnimInstance.JumpToNode` (`PaperZDAnimationComponent.AnimInstance` (`self.AnimationComponent`)) (`self.Ranged Attack Jump Node`) "None")
      (`SceneComponent.SetVisibility` (`self.Widget`) true false)
      (`KismetSystemLibrary.RetriggerableDelay` 1.0)
      (set `self.enemyDamaged` false))))

(event `self.Box.OnComponentBeginOverlap`
  (params (OverlappedComponent :type "PrimitiveComponent Object Reference") (OtherActor :type "Actor Object Reference") (OtherComp :type "PrimitiveComponent Object Reference") (OtherBodyIndex :type Integer) (bFromSweep :type Boolean) (SweepResult :type "HitResult Structure (by ref)"))
  ;[1 1 1] Handle Attack
  (if (== OtherActor (`GameplayStatics.GetPlayerCharacter` 0))
    (`KismetSystemLibrary.K2_SetTimerDelegate` (delegate `MushroomAttack`) 1.5 true false -1.5)))

(event `MushroomAttack`
  ;[1 1 1] Handle Attack
  (if (not (or (`self.isDead`) (`NavMovementComponent.IsFalling` (`self.CharacterMovement`))))
    (`PaperZDAnimInstance.JumpToNode` (`PaperZDAnimationComponent.AnimInstance` (`self.AnimationComponent`)) "Attack" "None")))

(event `SpawnProjectile`
  ;[1 1 1] Handle Attack
  (`|SpawnActorFromClass` (`self.Projectile`) (`KismetMathLibrary.MakeTransform` (`SceneComponent.K2_GetComponentLocation` (`self.SpawnPoint`)) (`self.K2_GetActorRotation`)) "Undefined" "MultiplyWithRoot" null null))

(fn `UserConstructionScript`)