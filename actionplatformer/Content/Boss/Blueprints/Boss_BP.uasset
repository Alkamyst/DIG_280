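; Side-scrolling boss character that turns toward the player, closes in along X until within range, and shows its own health bar.
; A random-interval looping timer triggers the attack animation, while a separate Attack event spawns a projectile aimed at the player.
; Damage updates health, knocks the boss back, briefly suppresses attacks, then restores flying movement.
; Death plays an animation, marks a level flag in the player's save, and opens the main menu.
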(event `self.ReceiveTick`
  (params (DeltaSeconds :type "Float (single-precision)"))
  (bind _returnvalue_x (`KismetMathLibrary.BreakVector` (- (`self.K2_GetActorLocation` (`GameplayStatics.GetPlayerCharacter` 0)) (`self.K2_GetActorLocation`))))
  (bind _returnvalue_x_2 (`KismetMathLibrary.BreakVector` (`KismetMathLibrary.Normal` (`KismetMathLibrary.MakeVector` _returnvalue_x))))
  (if (not (`self.isDead`))
    (`self.HandleRotation`)
    (if (not (< (`KismetMathLibrary.Abs` _returnvalue_x) 450.0))
      (`self.AddMovementInput` (1.0 0.0 0.0) _returnvalue_x_2))))

(event `HandleRotation`
  (bind _returnvalue_x (`KismetMathLibrary.BreakVector` (`KismetMathLibrary.GetDirectionUnitVector` (`self.K2_GetActorLocation` (`GameplayStatics.GetPlayerCharacter` 0)) (`self.K2_GetActorLocation`))))
  ;[1 1 1] Handle Rotation
  (if (`self.isDead`)
    _
    (elif (< _returnvalue_x 0.0)
      (`self.K2_SetActorRotation` (struct))
      (else
        (`self.K2_SetActorRotation` (struct :`Yaw` 180.0))))))

(event `self.ReceiveBeginPlay`
  (bind _returnvalue (`KismetSystemLibrary.K2_SetTimerDelegate` (delegate `PlayBossAttackAnimation`) (`KismetMathLibrary.RandomFloatInRange` 2.0 4.0) true))
  (set `self.bossAttackEvent` _returnvalue)
  (set `self.maxHealth` (`self.health`))
  (bind _returnvalue_2 (`|CreateWidget` "/Game/WidgetBlueprints/BossHealthBar_WBP.BossHealthBar_WBP_C" null self))
  (bind _output_get (set `self.BossHudRef` _returnvalue_2))
  (`UserWidget.AddToViewport` _output_get 0))

(event `PlayBossAttackAnimation`
  (if (not (or (`self.enemyDamaged`) (`self.isDead`)))
    (`PaperZDAnimInstance.JumpToNode` (`PaperZDAnimationComponent.AnimInstance` (`self.AnimationComponent`)) "Attack" "None")))

(event `Attack`
  (`SceneComponent.K2_SetWorldRotation` (`self.ProjectileSpawnLocation`) (`KismetMathLibrary.FindLookAtRotation` (`self.K2_GetActorLocation`) (`self.K2_GetActorLocation` (`GameplayStatics.GetPlayerCharacter` 0))) false false)
  (`|SpawnActorFromClass` "/Game/Boss/Blueprints/BossProjectile_BP.BossProjectile_BP_C" (`SceneComponent.K2_GetComponentToWorld` (`self.ProjectileSpawnLocation`)) "Undefined" "MultiplyWithRoot" null null))

(event `self.ReceiveAnyDamage`
  (params (Damage :type "Float (single-precision)") (DamageType :type "DamageType Object Reference") (InstigatedBy :type "Controller Object Reference") (DamageCauser :type "Actor Object Reference"))
  (bind _returnvalue_x (`KismetMathLibrary.BreakVector` (`KismetMathLibrary.GetDirectionUnitVector` (`self.K2_GetActorLocation` DamageCauser) (`self.K2_GetActorLocation`))))
  (if (not (`self.isDead`))
    (set `self.health` (- (`self.health`) Damage))
    (set `self.enemyDamaged` true)
    (`/Game/WidgetBlueprints/BossHealthBar_WBP.UpdateHealthBar` (`self.BossHudRef`))
    (`self.LaunchCharacter` (`KismetMathLibrary.MakeVector` (* (select `bool` (< _returnvalue_x 0.0) :`false` -1.0 :`true` 1.0) -800.0)) true true)
    (`|ExecutionSequence`
      (:`then_0`
        (if (<= (`self.health`) 0.0)
          (set `self.isDead` true)
          (`PaperZDAnimInstance.JumpToNode` (`PaperZDAnimationComponent.AnimInstance` (`self.AnimationComponent`)) "Die" "None")
          (`Widget.RemoveFromParent` (`self.BossHudRef`))
          (`KismetSystemLibrary.Delay` 2.0)
          (bind _asplayer_bp (cast `/Game/PlayerCharacter/Player_BP` (`GameplayStatics.GetPlayerCharacter` 0)))
          (bind _as_player_save (`/Game/PlayerCharacter/Player_BP.As Player Save` _asplayer_bp))
          (`KismetArrayLibrary.Array_Set` (`/Game/PlayerCharacter/PlayerSave.levels` _as_player_save) 2 true)
          (`GameplayStatics.SaveGameToSlot` _as_player_save "1")
          (`GameplayStatics.OpenLevel` "MainMenuMap")
          (else
            (`PaperZDAnimInstance.JumpToNode` (`PaperZDAnimationComponent.AnimInstance` (`self.AnimationComponent`)) "Damaged" "None")
            (`KismetSystemLibrary.RetriggerableDelay` 1.0)
            (set `self.enemyDamaged` false))))
      (:`then_1`
        (`KismetSystemLibrary.Delay` 0.7)
        (`CharacterMovementComponent.SetMovementMode` (`self.CharacterMovement`) "MOVE_Flying" 0)))))

(fn `UserConstructionScript`)