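; Side-scrolling skeleton enemy character that patrols along the X axis and attacks the player.
; Tick drives movement and facing, with forward and downward line traces triggering a pause and turn at obstacles or ledges.
; A Box overlap halts patrol and loops attack animations by timer, while a separate Attack event traces to damage the player.
; Damage updates a health bar widget, then knocks the skeleton back or plays death before destroying it.
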(event `self.ReceiveBeginPlay`
  (set `self.Max Walk Speed` (`self.Max Walk Speed`))
  (set `self.maxHealth` (`self.Health`))
  (bind _asenemy_health_bar_wbp (cast `/Game/WidgetBlueprints/EnemyHealthBar_WBP` (`WidgetComponent.GetWidget` (`self.Widget`))))
  (set `/Game/WidgetBlueprints/EnemyHealthBar_WBP.skeletonRef` self _asenemy_health_bar_wbp)
  (set `self.As Enemy Health Bar WBP` _asenemy_health_bar_wbp))

(event `self.ReceiveTick`
  (params (DeltaSeconds :type "Float (single-precision)"))
  (`self.Handle Rotation`)
  (`self.HandleMovement`))

(event `HandleMovement`
  (bind _returnvalue (`self.K2_GetActorLocation`))
  (bind _returnvalue_2 (`self.K2_GetActorLocation`))
  ;[1 1 1] Handle Movement
  (if (not (or (`self.isDead`) (`self.enemyDamaged`) (`NavMovementComponent.IsFalling` (`self.CharacterMovement`)) (`self.attackMode`)))
    (`self.AddMovementInput` (1.0 0.0 0.0) (`self.Movement Direction`))
    (`|ExecutionSequence`
      (:`then_0`
        ;;[1 1 1] Detect if Something is in Front of Skeleton
        (bind (_outhit _returnvalue_3) (`KismetSystemLibrary.LineTraceSingleForObjects` _returnvalue (+ _returnvalue (* (`self.GetActorForwardVector`) (100.0 0.0 0.0))) (`|MakeArray` "ObjectTypeQuery1" "ObjectTypeQuery2" "ObjectTypeQuery3" :!type "EObjectTypeQuery Enum") false (`|MakeArray` (`GameplayStatics.GetPlayerCharacter` 0) :!type "Actor Object Reference")))
        (if _returnvalue_3
          (`/Engine/EditorBlueprintResources/StandardMacros.DoOnce` false :!label _label
            (:`Completed`
              (set `CharacterMovementComponent.MaxWalkSpeed` 0.0 (`self.CharacterMovement`))
              (`KismetSystemLibrary.Delay` (`self.Wait Time`))
              (set `CharacterMovementComponent.MaxWalkSpeed` (`self.Max Walk Speed`) (`self.CharacterMovement`))
              (set `self.Movement Direction` (* (`self.Movement Direction`) -1.0))
              (goto _label :!via `Reset`)))))
      (:`then_1`
        ;;[1 1 1] Detect if Skeleton has reached an Edge
        (bind (_outhit_2 _returnvalue_4) (`KismetSystemLibrary.LineTraceSingleForObjects` _returnvalue_2 (+ (- _returnvalue_2 (0.0 0.0 100.0)) (* (`self.GetActorForwardVector`) (100.0 0.0 0.0))) (`|MakeArray` "ObjectTypeQuery1" "ObjectTypeQuery2" "ObjectTypeQuery3" :!type "EObjectTypeQuery Enum") false (`|MakeArray` (`GameplayStatics.GetPlayerCharacter` 0) :!type "Actor Object Reference")))
        (if (not _returnvalue_4)
          (goto _label))))))

(event `Handle Rotation`
  ;[1 1 1] Handle Rotation
  (if (> (`self.Movement Direction`) 0.0)
    (`self.K2_SetActorRotation` (struct))
    (else
      (`self.K2_SetActorRotation` (struct :`Yaw` 180.0)))))

(event `self.ReceiveAnyDamage`
  (params (Damage :type "Float (single-precision)") (DamageType :type "DamageType Object Reference") (InstigatedBy :type "Controller Object Reference") (DamageCauser :type "Actor Object Reference"))
  (bind _returnvalue_x (`KismetMathLibrary.BreakVector` (`KismetMathLibrary.GetDirectionUnitVector` (`self.K2_GetActorLocation` DamageCauser) (`self.K2_GetActorLocation`))))
  (bind _returnvalue (select `bool` (< _returnvalue_x 0.0) :`false` -1.0 :`true` 1.0))
  ;[1 1 1] Handle Damage
  (if (not (`self.isDead`))
    (bind _output_get (set `self.Health` (- (`self.Health`) Damage)))
    (set `self.enemyDamaged` true)
    (set `self.Movement Direction` _returnvalue)
    (`/Game/WidgetBlueprints/EnemyHealthBar_WBP.UpdateHealthBar` (`self.As Enemy Health Bar WBP`))
    (if (<= _output_get 0.0)
      (`PaperZDAnimInstance.JumpToNode` (`PaperZDAnimationComponent.AnimInstance` (`self.AnimationComponent`)) "Death" "None")
      (set `self.isDead` true)
      (`PrimitiveComponent.SetCollisionProfileName` (`self.CapsuleComponent`) (`self.Death Jump Node`) true)
      (`SceneComponent.SetVisibility` (`self.Widget`) false false)
      (`KismetSystemLibrary.Delay` 3.0)
      (`self.K2_DestroyActor`)
      (else
        (`self.LaunchCharacter` (`KismetMathLibrary.MakeVector` (* _returnvalue -800.0) 0.0 150.0) true true)
        (`PaperZDAnimInstance.JumpToNode` (`PaperZDAnimationComponent.AnimInstance` (`self.AnimationComponent`)) (`self.Damaged Jump Node`) "None")
        (`SceneComponent.SetVisibility` (`self.Widget`) true false)
        (`KismetSystemLibrary.RetriggerableDelay` 1.0)
        (set `self.enemyDamaged` false)))))

(event `self.Box.OnComponentBeginOverlap`
  (params (OverlappedComponent :type "PrimitiveComponent Object Reference") (OtherActor :type "Actor Object Reference") (OtherComp :type "PrimitiveComponent Object Reference") (OtherBodyIndex :type Integer) (bFromSweep :type Boolean) (SweepResult :type "HitResult Structure (by ref)"))
  ;[1 1 1] Handle Attack System
  (if (== OtherActor (`GameplayStatics.GetPlayerCharacter` 0))
    (set `self.attackMode` true)
    (bind _returnvalue (`KismetSystemLibrary.K2_SetTimerDelegate` (delegate `Skeleton Attack`) 1.0 true false -1.0))
    (set `self.attackEvent` _returnvalue)))

(event `Skeleton Attack`
  ;[1 1 1] Handle Attack System
  (if (not (`self.isDead`))
    (`PaperZDAnimInstance.JumpToNode` (`PaperZDAnimationComponent.AnimInstance` (`self.AnimationComponent`)) (`self.Attack Jump Node`) "None")))

(event `self.Box.OnComponentEndOverlap`
  (params (OverlappedComponent :type "PrimitiveComponent Object Reference") (OtherActor :type "Actor Object Reference") (OtherComp :type "PrimitiveComponent Object Reference") (OtherBodyIndex :type Integer))
  ;[1 1 1] Handle Attack System
  (if (== OtherActor (`GameplayStatics.GetPlayerCharacter` 0))
    (set `self.attackMode` false)
    (`KismetSystemLibrary.K2_ClearAndInvalidateTimerHandle` (`self.attackEvent`))))

(event `Attack`
  (bind _returnvalue (`self.K2_GetActorLocation`))
  ;[1 1 1] Handle Attack System
  (bind _outhit (`KismetSystemLibrary.LineTraceSingleForObjects` _returnvalue (+ (* (`self.GetActorForwardVector`) (200.0 0.0 0.0)) _returnvalue) (`|MakeArray` "ObjectTypeQuery3" :!type "EObjectTypeQuery Enum")))
  (bind (_bblockinghit _binitialoverlap _time _distance _location _impactpoint _normal _impactnormal _physmat _hitactor) (`GameplayStatics.BreakHitResult` _outhit))
  (if (== _hitactor (`GameplayStatics.GetPlayerCharacter` 0))
    (`GameplayStatics.ApplyDamage` _hitactor 1.0)))

(fn `UserConstructionScript`)